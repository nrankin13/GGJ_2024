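; BP_Missile is a projectile that flies toward the player's position and ragdolls the third-person character it hits.
; On BeginPlay it samples the player controller's location once and rotates to face it, so it does not home afterward.
; Tick lerps from its current location toward a point below that snapshot with a growing alpha, accelerating the approach.
; Tick also polls the Collider's overlaps, calling Ragdoll on the character and destroying the missile.
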(event `self.ReceiveBeginPlay`
  (bind _output_get (set `self.PlayerLocation` (`self.K2_GetActorLocation` (`GameplayStatics.GetPlayerController` 0))))
  (`self.K2_SetActorRotation` (`KismetMathLibrary.FindLookAtRotation` (`self.K2_GetActorLocation`) _output_get)))

(event `self.ReceiveTick`
  (params (DeltaSeconds :type "Float (single-precision)"))
  (bind _output_get (set `self.Alpha` (+ (`self.Alpha`) (/ DeltaSeconds 5.0))))
  (`self.K2_SetActorLocation` (`KismetMathLibrary.VLerp` (`self.K2_GetActorLocation`) (- (`self.PlayerLocation`) (0.0 0.0 90.0)) _output_get))
  (for _array_element (`PrimitiveComponent.GetOverlappingActors` (`self.Collider`) "/Game/ThirdPerson/Blueprints/BP_ThirdPersonCharacter.BP_ThirdPersonCharacter_C")
    (bind _asbp_third_person_character (cast `/Game/ThirdPerson/Blueprints/BP_ThirdPersonCharacter` _array_element))
    (`/Game/ThirdPerson/Blueprints/BP_ThirdPersonCharacter.Ragdoll` _asbp_third_person_character)
    (`self.K2_DestroyActor`)))

(fn `UserConstructionScript`)