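; Alien ship pawn that roams the level on its own and randomly spawns pickup crates along the way.
; From BeginPlay it loops: pick a random navigable point within a radius of itself, then fly there with AI MoveTo.
; On arrival it has a 50% chance to spawn a BP_PickUpCrate offset above its position, then waits briefly before repeating.
; A failed move retries immediately with a new point.
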(event `FlyRandomly`
  (bind _randomlocation (`NavigationSystemV1.K2_GetRandomLocationInNavigableRadius` (`self.K2_GetActorLocation`) 5000.0 null null :!label _label))
  (`KismetSystemLibrary.PrintString` "Hello")
  (`|AIMoveTo` self _randomlocation null
    (:`OnSuccess`
      (if (> (`KismetMathLibrary.RandomFloat`) 0.5)
        (`|SpawnActorFromClass` "/Game/BP_PickUpCrate.BP_PickUpCrate_C" (`KismetMathLibrary.MakeTransform` (- (.location (`self.GetTransform`)) (0.0 0.0 -1500.0)) (.rotation (`self.GetTransform`))) "AlwaysSpawn" "MultiplyWithRoot" null null))
      (`KismetSystemLibrary.Delay` 2.0)
      (`self.FlyRandomly`))
    (:`OnFail`
      (`self.FlyRandomly`))))

(event `self.ReceiveBeginPlay`
  (goto _label))

(fn `UserConstructionScript`)