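; BP_PickUpCrate is a physics crate that homes in on the player pawn.
; Shortly after BeginPlay, a DelayUntilNextTick loop replaces Tick, pushing the StaticMesh toward the player every frame with a constant, mass-independent force.
; The Hit event is empty; disconnected DoOnce logic that would spawn BP_ExplodingActors at the hit location and destroy the crate never runs.
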(event `self.ReceiveBeginPlay`
  (`KismetSystemLibrary.Delay` 0.1)
  (`PrimitiveComponent.AddForce` (`self.StaticMesh`) (* (`KismetMathLibrary.Normal` (- (`self.K2_GetActorLocation` (`GameplayStatics.GetPlayerPawn` 0)) (`self.K2_GetActorLocation`))) 8000.0) "None" true :!label _label)
  (`KismetSystemLibrary.DelayUntilNextTick`)
  (goto _label))

(event `self.ReceiveHit`
  (params (MyComp :type "PrimitiveComponent Object Reference") (Other :type "Actor Object Reference") (OtherComp :type "PrimitiveComponent Object Reference") (bSelfMoved :type Boolean) (HitLocation :type "Vector Structure") (HitNormal :type "Vector Structure") (NormalImpulse :type "Vector Structure") (Hit :type "HitResult Structure (by ref)")))

(fn `UserConstructionScript`)