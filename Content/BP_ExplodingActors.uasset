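; BP_ExplodingActors is a spawner that fills a cubic grid with BP_RubberDuck actors when play begins.
; SpawnActors derives the grid's side from the rounded-up cube root of AmountToSpawn, so the actual count only approximates that value.
; Three nested loops place ducks at fixed spacing from the spawner's location, always spawning regardless of collision.
; Despite the name, this Blueprint contains no explosion logic.
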(event `self.ReceiveBeginPlay`
  (`self.SpawnActors` (`self.AmountToSpawn`)))

(fn `SpawnActors`
  (params (AmountToSpawn :type Integer))
  (locals (X :type Integer) (Y :type Integer) (Z :type Integer))
  (bind _returnvalue (`KismetMathLibrary.FCeil` (`KismetMathLibrary.MultiplyMultiply_FloatFloat` (`KismetMathLibrary.Conv_IntToDouble` AmountToSpawn) 0.333333)))
  (for _index (range (+ _returnvalue 1))
    (set `local.X` _index)
    (for _index_2 (range (+ _returnvalue 1))
      (set `local.Y` _index_2)
      (for _index_3 (range (+ _returnvalue 1))
        (set `local.Z` _index_3)
        (`|SpawnActorFromClass` "/Game/BP_RubberDuck.BP_RubberDuck_C" (`KismetMathLibrary.MakeTransform` (+ (`KismetMathLibrary.MakeVector` (`KismetMathLibrary.Conv_IntToDouble` (* (`local.X`) 40)) (`KismetMathLibrary.Conv_IntToDouble` (* (`local.Y`) 40)) (`KismetMathLibrary.Conv_IntToDouble` (* (`local.Z`) 40))) (`self.K2_GetActorLocation`))) "AlwaysSpawn" "MultiplyWithRoot" null null)))))

(fn `UserConstructionScript`)